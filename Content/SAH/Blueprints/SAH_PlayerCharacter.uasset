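; Player character Blueprint that maps input to inherited combat actions: attacks, dodges, dashes, counters, blocking and job switching.
; Tick runs stamina regen, armor regen and combo timing, then refreshes the health, armor and stamina bars of a HUD widget created at BeginPlay alongside a debug widget.
; Debug keys trigger enemy attacks, change health, test blocked damage, set status and spawn attack actors that hit the player.
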(event EventBeginPlay
  (|CallParentFunction)
  (CallFunction|SetUI))

(event Collision|EventActorBeginOverlap
  (params (OtherActor :type Actor%20Object%20Reference)))

(event EventTick
  (params (DeltaSeconds :type Float%20%28single-precision%29))
  (CallFunction|StaminaRegenTiming DeltaSeconds)
  (CallFunction|ArmorRegenTiming DeltaSeconds)
  (CallFunction|ComboTiming DeltaSeconds)
  (CallFunction|UpdateGUI))

(event Input|ActionEvents|InputActionPrimaryAttack
  (params (Key :type Key%20Structure :default "AnyKey"))
  ;[1 1 1] Attack action
  (:Pressed
    (CallFunction|Attack true)))

(event Input|ActionEvents|InputActionSecondaryAttack
  (params (Key :type Key%20Structure :default "AnyKey"))
  ;[1 1 1] Attack action
  (:Pressed
    (CallFunction|Attack false)))

(event Input|ActionEvents|InputActionBlock
  (params (Key :type Key%20Structure :default "AnyKey"))
  ;[1 1 1] Blocking actions
  (:Pressed
    (CallFunction|StartBlock))
  (:Released
    (CallFunction|StopBlock)))

(event Input|ActionEvents|InputActionDodgeDown
  (params (Key :type Key%20Structure :default "AnyKey"))
  ;[1 1 1] Blocking actions
  (:Pressed
    (CallFunction|DodgeDown)))

(event Input|ActionEvents|InputActionDodgeUp
  (params (Key :type Key%20Structure :default "AnyKey"))
  ;[1 1 1] Blocking actions
  (:Pressed
    (CallFunction|DodgeUp)))

(event Input|ActionEvents|InputActionDashForward
  (params (Key :type Key%20Structure :default "AnyKey"))
  ;[1 1 1] Blocking actions
  (:Pressed
    (CallFunction|Dash 1.0)))

(event Input|ActionEvents|InputActionDashBackward
  (params (Key :type Key%20Structure :default "AnyKey"))
  ;[1 1 1] Blocking actions
  (:Pressed
    (CallFunction|Dash -1.0)))

(event Input|ActionEvents|InputActionPrimaryCounter
  (params (Key :type Key%20Structure :default "AnyKey"))
  ;[1 1 1] Blocking actions
  (:Pressed
    (CallFunction|TryCounter (Variables|/Game/SAH/ATS/ATS_base.ATS_base_C|Gettype (Utilities|Array|Get(acopy) (Variables|Default|Getprimary))))))

(event Input|ActionEvents|InputActionSecondaryCounter
  (params (Key :type Key%20Structure :default "AnyKey"))
  ;[1 1 1] Blocking actions
  (:Pressed
    (CallFunction|TryCounter (Variables|/Game/SAH/ATS/ATS_base.ATS_base_C|Gettype (Utilities|Array|Get(acopy) (Variables|Default|Getsecondary))))))

(event Input|ActionEvents|InputActionChangeNext
  (params (Key :type Key%20Structure :default "AnyKey"))
  ;[1 1 1] Job actions
  (:Pressed
    (bind _newindex (CallFunction|UpdateJobIndex 1))
    (Variables|Default|SetnewJob _newindex)
    (CallFunction|StartChangeJob)))

(event Input|ActionEvents|InputActionChangePrevious
  (params (Key :type Key%20Structure :default "AnyKey"))
  ;[1 1 1] Job actions
  (:Pressed
    (bind _newindex (CallFunction|UpdateJobIndex -1))
    (Variables|Default|SetnewJob _newindex)
    (CallFunction|StartChangeJob)))

(event Input|KeyboardEvents|U
  (params (Key :type Key%20Structure :default "AnyKey"))
  ;[1 1 1] Debug
  ;;[1 1 1] Modify the character stats
  (:Pressed
    (Variables|Default|SetStatus "NewEnumerator0")))

(event Input|KeyboardEvents|Alt1
  (params (Key :type Key%20Structure :default "AnyKey"))
  (bind _self self)
  ;[1 1 1] Debug
  ;;[1 1 1] Simulate an enemy attack
  (:Pressed
    (bind _returnvalue (Game|SpawnActorfromClass "/Game/SAH/ATS/ATS_AJ_slash_1.ATS_AJ_slash_1_C" (Transformation|GetActorTransform) "AdjustIfPossibleButDontSpawnIfColliding" 0 0))
    (Default|DealDamage _returnvalue _self _self)))

(event Input|KeyboardEvents|Alt2
  (params (Key :type Key%20Structure :default "AnyKey"))
  (bind _self self)
  ;[1 1 1] Debug
  ;;[1 1 1] Simulate an enemy attack
  (:Pressed
    (bind _returnvalue (Game|SpawnActorfromClass "/Game/SAH/ATS/ATS_AJ_slash_2.ATS_AJ_slash_2_C" (Transformation|GetActorTransform) "AdjustIfPossibleButDontSpawnIfColliding" 0 0))
    (Default|DealDamage _returnvalue _self _self)))

(event Input|KeyboardEvents|G
  (params (Key :type Key%20Structure :default "AnyKey"))
  ;[1 1 1] Debug
  ;;[1 1 1] Modify the character stats
  (:Pressed
    (CallFunction|Heal 1.0)))

(event Input|KeyboardEvents|C
  (params (Key :type Key%20Structure :default "AnyKey"))
  ;[1 1 1] Debug
  ;;[1 1 1] Modify the character stats
  (:Pressed
    (CallFunction|TakeDamage 1.0)))

(event Input|KeyboardEvents|V
  (params (Key :type Key%20Structure :default "AnyKey"))
  ;[1 1 1] Debug
  (:Pressed
    (bind _newdamage (CallFunction|BlockDamage 1.0))
    (CallFunction|TakeDamage _newdamage)))

(event Input|KeyboardEvents|B
  (params (Key :type Key%20Structure :default "AnyKey"))
  ;[1 1 1] Debug
  (:Pressed
    (bind _outactors (Actor|GetAllActorsOfClass "/Game/SAH/Blueprints/SAH_EnemyCharacter.SAH_EnemyCharacter_C"))
    (if (Utilities|IsValid (Utilities|Array|Get(acopy) _outactors))
      (Default|Attack (Utilities|Array|Get(acopy) _outactors) true))))

(fn ConstructionScript
  (|CallParentFunction))

(fn SetUI
  (bind _returnvalue (UserInterface|CreateWidget "/Game/SAH/UI/SAH_debug.SAH_debug_C"))
  (bind _output_get (Variables|Default|SetDebugHUD _returnvalue))
  (UserInterface|Viewport|AddtoViewport _output_get 0)
  (bind _returnvalue_2 (UserInterface|CreateWidget "/Game/SAH/UI/SAH_PlayerBars.SAH_PlayerBars_C"))
  (bind _output_get_2 (Variables|Default|SetbarsHUD _returnvalue_2))
  (UserInterface|Viewport|AddtoViewport _output_get_2 0)
  (return))

(fn UpdateGUI
  (bind _stats (Variables|Default|Getstats))
  (bind _barshud (Variables|Default|GetbarsHUD))
  (bind (_healthmax _staminamax _staminaregen _armormax) (Utilities|Struct|BreakSStats _stats))
  (Progress|SetPercent (Variables|/Game/SAH/UI/SAH_PlayerBars.SAH_PlayerBars_C|GethealthBar _barshud) (/ (Variables|Default|Gethealth) _healthmax))
  (Progress|SetPercent (Variables|/Game/SAH/UI/SAH_PlayerBars.SAH_PlayerBars_C|GetarmorBar _barshud) (/ (Variables|Default|Getarmor) _armormax))
  (Progress|SetPercent (Variables|/Game/SAH/UI/SAH_PlayerBars.SAH_PlayerBars_C|GetstaminaBar _barshud) (/ (Variables|Default|Getstamina) _staminamax)))