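; Enemy character Blueprint that starts with full health, stamina and armor and displays them on status bars.
; On BeginPlay it runs the parent logic, adds an SAH_EnemyDebug widget to the viewport, then sets each stat to its maximum from Stats.
; Every tick it casts a user widget object to SAH_bars and sets the three bars to current-to-maximum ratios.
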(event EventBeginPlay
  (bind _stats (Variables|Default|Getstats))
  (bind (_healthmax _staminamax _staminaregen _armormax) (Utilities|Struct|BreakSStats _stats))
  (|CallParentFunction)
  (Build|SetEnemyUI)
  ;[1 1 1] Unlike the player character, the enemy start with all its health
  (Variables|Default|Sethealth _healthmax)
  (Variables|Default|Setstamina _staminamax)
  (Variables|Default|Setarmor _armormax))

(event Collision|EventActorBeginOverlap
  (params (OtherActor :type Actor%20Object%20Reference)))

(event EventTick
  (params (DeltaSeconds :type Float%20%28single-precision%29))
  (|CallParentFunction 0.0)
  (CallFunction|UpdateGUI))

(fn ConstructionScript
  (|CallParentFunction))

(fn SetEnemyUI
  (bind _returnvalue (UserInterface|CreateWidget "/Game/SAH/UI/SAH_EnemyDebug.SAH_EnemyDebug_C"))
  (bind _output_get (Variables|Default|SetUI _returnvalue))
  (UserInterface|Viewport|AddtoViewport _output_get 0)
  (return))

(fn UpdateGUI
  (bind _stats (Variables|Default|Getstats))
  (bind (_healthmax _staminamax _staminaregen _armormax) (Utilities|Struct|BreakSStats _stats))
  (bind _assah_bars (Utilities|Casting|CastToSAH_bars (UserInterface|GetUserWidgetObject)))
  (Progress|SetPercent (Variables|/Game/SAH/UI/SAH_bars.SAH_bars_C|GethealthBar _assah_bars) (/ (Variables|Default|Gethealth) _healthmax))
  (Progress|SetPercent (Variables|/Game/SAH/UI/SAH_bars.SAH_bars_C|GetarmorBar _assah_bars) (/ (Variables|Default|Getarmor) _armormax))
  (Progress|SetPercent (Variables|/Game/SAH/UI/SAH_bars.SAH_bars_C|GetstaminaBar _assah_bars) (/ (Variables|Default|Getstamina) _staminamax)))