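; Healing fountain actor that periodically heals player characters standing within its overlap area.
; Overlap events track characters in a list, and each entry switches the flipbook to healing and sets a looping timer that heals everyone listed.
; Tick polls the list every frame, restoring the idle flipbook and clearing the timer whenever it is empty.
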(event EventBeginPlay)

(event EventActorBeginOverlap
  (params (OtherActor :type Actor%20Object%20Reference))
  (bind _assah_player_character (Utilities|Casting|CastToSAH_PlayerCharacter OtherActor))
  (Utilities|Array|AddUnique (Variables|Default|GetcurrentCharacters) _assah_player_character)
  (Sprite|SetFlipbook (Variables|Default|Getbody) (Variables|Default|GetBook_healing))
  (Utilities|Time|SetTimerbyFunctionName 0 "HealCharacters" (Variables|Default|GethealingRate) true))

(event EventTick
  (params (DeltaSeconds :type Float%20%28single-precision%29))
  (if (<= (Utilities|Array|Length (Variables|Default|GetcurrentCharacters)) 0)
    (Sprite|SetFlipbook (Variables|Default|Getbody) (Variables|Default|GetBook_idle))
    (Utilities|Time|ClearTimerbyFunctionName 0 "HealCharacters")))

(event EventActorEndOverlap
  (params (OtherActor :type Actor%20Object%20Reference))
  (bind _assah_player_character (Utilities|Casting|CastToSAH_PlayerCharacter OtherActor))
  (Utilities|Array|RemoveItem (Variables|Default|GetcurrentCharacters) _assah_player_character))

(fn ConstructionScript)

(fn HealCharacters
  (for _array_element (Variables|Default|GetcurrentCharacters)
    (Default|Heal _array_element (Variables|Default|GethealValue))))